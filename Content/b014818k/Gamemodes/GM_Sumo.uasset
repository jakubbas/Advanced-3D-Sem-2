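; Sumo game mode built on a parent mode, where the last remaining player's team takes the score.
; On death, a player's widget and pawn are removed, and their controller possesses a spawned spectator.
; When one player remains, that player's team is passed to the score update.
; A timer boosts every player's power at four set intervals, and Clear sends a zero power value before calling the parent's cleanup.
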(event `self.ReceiveBeginPlay`
  (`self.Init`))

(event `/Game/b014818k/Blueprints/Interfaces/BPI_Player.I_PlayerDeath`
  (params (Controller :type "Controller Object Reference"))
  (bind _returnvalue (`Controller.K2_GetPawn` Controller))
  ;[1 0.237 0.6461] On player death Clear the widget, remove from player array and destroy, and then create and possess a spectator pawn.
  (bind _playerwidget (message `/Game/b014818k/Blueprints/Interfaces/BPI_PlayerUI.I_GetPlayerWidget` _returnvalue))
  (`Widget.RemoveFromParent` _playerwidget)
  (bind _character (message `/Game/b014818k/Blueprints/Interfaces/BPI_BasicPlayer.I_GetCharacter` _returnvalue))
  (`self.ClearPawn` _character)
  (bind _returnvalue_2 (`|SpawnActorFromClass` "/Game/b014818k/Blueprints/Characters/SpectatorPlayer/CH_Spectator.CH_Spectator_C" (`self.GetTransform` _returnvalue) "AlwaysSpawn" "OverrideRootScale" null null))
  (`self.K2_DestroyActor` _returnvalue)
  (message `/Game/b014818k/Blueprints/Interfaces/BPI_BaseGM.I_SetPawn` Controller _returnvalue_2)
  (`Controller.Possess` Controller _returnvalue_2)
  (`KismetArrayLibrary.Array_Add` (`self.Spectators`) _returnvalue_2)
  (if (== 1 (`KismetArrayLibrary.Array_Length` (`self.Players`)))
    (bind _winningteam (`self.AllPlayersFinished`))
    (`self.UpdateGameScore` _winningteam)))

(fn `AllPlayersFinished`
  (returns (WinningTeam :type "/Game/b014818k/Blueprints/Enumerators/Enum_Teams Enum"))
  (for _array_element (`self.Players`)
    (return (`.Team_3_5BCB2BAE40BA236510DE158E7B2C8C60` (break `/Game/b014818k/Blueprints/Structs/Struct_Scores` (`|GetArrayItem` (`self.ScoresStruct`) (`KismetArrayLibrary.Array_Find` (`self.Controllers`) (`Pawn.GetController` _array_element))))))))

(fn `Clear`
  (for _array_element (`self.Players`)
    (`/Engine/EditorBlueprintResources/StandardMacros.IsValid` _array_element
      (:`Is Valid`
        (message `/Game/b014818k/Blueprints/Interfaces/BPI_Player.I_IncreasePower` _array_element 0.0))
      (:`Is Not Valid`
        _))
    (`parent.Clear`)))

(fn `I_IsSumoGM`
  (returns (IsSumoGm :type Boolean))
  (return true))

(fn `Timer`
  (`/Engine/EditorBlueprintResources/StandardMacros.IncrementInt` (`self.Time`)
    (:`  `
      (if (or (== (`self.Time`) 15) (== (`self.Time`) 30) (== (`self.Time`) 45) (== (`self.Time`) 60))
        (for _array_element (`self.Players`)
          (message `/Game/b014818k/Blueprints/Interfaces/BPI_Player.I_IncreasePower` _array_element 1.25))))))

(fn `UserConstructionScript`
  (`parent.UserConstructionScript`))
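; Game mode for the DeathRun minigame, which pits one DeathRun character against the remaining basic players.
; BeginPlay prints the map and mode, then runs Init.
; SpawnCharacters gives the first controller CH_DeathRun at a fixed location and the others CH_BasicPlayer at unoccupied spawns.
; ScreenCover, ChangeMovement and Countdown apply fades, movement toggling and countdown to the DeathRun player, then call the parent versions.
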(event `self.ReceiveBeginPlay`
  (bind _returnvalue (`GameplayStatics.GetCurrentLevelName` true))
  (`KismetSystemLibrary.PrintString` (`KismetStringLibrary.Concat_StrStr` "Map: " _returnvalue "" "Gamemode: " (`KismetSystemLibrary.GetDisplayName` (`GameplayStatics.GetGameMode`))))
  (`self.Init`))

(event `self.SpawnCharacters`
  ;[0.2486 0.2218 1] Spawns Main Menu Characters
  (for (_array_element _array_index) (`self.Controllers`)
    (if (== _array_index 0)
      (bind _returnvalue (`|SpawnActorFromClass` "/Game/b014818k/Blueprints/Characters/DeathrunPlayer/CH_DeathRun.CH_DeathRun_C" (`KismetMathLibrary.MakeTransform` (-200.0 0.0 100.0)) "Undefined" "OverrideRootScale" null null))
      (bind _output_get (set `self.DeathRunPlayer` _returnvalue))
      (message `/Game/b014818k/Blueprints/Interfaces/BPI_BaseGM.I_SetPawn` _array_element _output_get)
      (`Controller.Possess` _array_element _returnvalue)
      (else
        (bind _spawn (`self.FindUnoccupiedSpawn`))
        (bind _returnvalue_2 (`|SpawnActorFromClass` "/Game/b014818k/Blueprints/Characters/BasicPlayer/CH_BasicPlayer.CH_BasicPlayer_C" _spawn "Undefined" "OverrideRootScale" null null))
        (`KismetArrayLibrary.Array_Add` (`self.Players`) _returnvalue_2)
        (message `/Game/b014818k/Blueprints/Interfaces/BPI_BaseGM.I_SetPawn` _array_element _returnvalue_2)
        (`Controller.Possess` _array_element _returnvalue_2)))))

(event `self.PlayersAdded`)

(fn `ChangeMovement`
  (params (CanMove :type Boolean))
  (bind _charactermovement (`Character.CharacterMovement` (`self.DeathRunPlayer`)))
  (if CanMove
    (`ActorComponent.SetActive` _charactermovement true false)
    (else
      (`ActorComponent.SetActive` _charactermovement false false)))
  (`parent.ChangeMovement` CanMove))

(fn `Countdown`
  (message `/Game/b014818k/Blueprints/Interfaces/BPI_PlayerUI.I_Countdown` (`/Game/b014818k/Blueprints/Characters/DeathrunPlayer/CH_DeathRun.DeathRunWidget` (`self.DeathRunPlayer`)))
  (`parent.Countdown`))

(fn `ScreenCover`
  (params (CoverScreen :type Boolean) (Speed :type "Float (double-precision)"))
  (bind _deathrunwidget (`/Game/b014818k/Blueprints/Characters/DeathrunPlayer/CH_DeathRun.DeathRunWidget` (`self.DeathRunPlayer`)))
  (if CoverScreen
    (message `/Game/b014818k/Blueprints/Interfaces/BPI_PlayerUI.I_FadeIn` _deathrunwidget 1.0 "Forward")
    (else
      (message `/Game/b014818k/Blueprints/Interfaces/BPI_PlayerUI.I_FadeIn` _deathrunwidget 1.0 "Reverse")))
  (`parent.ScreenCover` CoverScreen Speed))

(fn `UserConstructionScript`
  (`parent.UserConstructionScript`))
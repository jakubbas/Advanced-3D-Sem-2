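; Base game mode for local multiplayer that creates players, spawns their characters and assigns teams.
; Init rebuilds local players from the PlayerCount URL option, possesses a CH_BasicPlayer for each controller, then sets teams by controller index, up to four.
; Spawns come from randomly picked BP_PlayerSpawn actors, which are invalidated and removed once used.
; LoadLevel carries game mode and player count through travel options; ReturnToMenu removes players and opens StartingMap.
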(event `Init`
  ;[0 1 0.0615] Initialises
  (`self.RemoveOtherPlayers`)
  (`self.Set Up Controllers` (`GameplayStatics.GetIntOption` (`self.OptionsString`) "PlayerCount" 1))
  (`self.GetSpawnLocations`)
  (`self.Spawn Characters`)
  (`self.Players Added`)
  (`self.Add To Team`))

(event `Set Up Controllers`
  (params (`Player Count` :type Integer))
  ;[0.2954 0.1818 1] Sets up the Player Controllers
  (for _index (range `Player Count`)
    (`GameplayStatics.CreatePlayer` _index)))

(event `RemoveOtherPlayers`
  ;[1 0.01995 0.05975] Removes all but 1 Player
  (for _index (range (`self.PlayerCount`))
    (bind _returnvalue (`GameplayStatics.GetPlayerControllerFromID` _index))
    (`/Engine/EditorBlueprintResources/StandardMacros.IsValid` _returnvalue
      (:`Is Valid`
        (`GameplayStatics.RemovePlayer` _returnvalue true)))))

(event `self.K2_PostLogin`
  (params (NewPlayer :type "PlayerController Object Reference"))
  ;[1 0.01201 0.4227] Adds and Removes Controllers from the array
  (`KismetArrayLibrary.Array_Add` (`self.Controllers`) NewPlayer))

(event `self.K2_OnLogout`
  (params (ExitingController :type "Controller Object Reference"))
  ;[1 0.01201 0.4227] Adds and Removes Controllers from the array
  (`KismetArrayLibrary.Array_RemoveItem` (`self.Controllers`) ExitingController))

(event `ReturnToMenu`
  (`self.RemoveOtherPlayers`)
  (`GameplayStatics.OpenLevel` "StartingMap"))

(event `LoadLevel`
  (params (Level :type Name) (Gamemode :type String))
  (`GameplayStatics.OpenLevel` Level true (`KismetStringLibrary.Concat_StrStr` "game=" Gamemode "?PlayerCount=" (`KismetStringLibrary.Conv_IntToString` (`self.PlayerCount`)))))

(event `Add To Team`
  ;[1 1 1] Add Players to Teams
  (for (_array_element _array_index) (`self.Controllers`)
    (switch `int` _array_index
      (:`0`
        (bind _returnvalue (`Controller.K2_GetPawn` _array_element))
        (message `/Game/b014818k/Blueprints/Interfaces/BPI_Teams.I_SetTeam` _returnvalue "NewEnumerator0"))
      (:`1`
        (message `/Game/b014818k/Blueprints/Interfaces/BPI_Teams.I_SetTeam` _returnvalue "NewEnumerator1"))
      (:`2`
        (bind _returnvalue_2 (`Controller.K2_GetPawn` _array_element))
        (message `/Game/b014818k/Blueprints/Interfaces/BPI_Teams.I_SetTeam` _returnvalue_2 "NewEnumerator3"))
      (:`3`
        (message `/Game/b014818k/Blueprints/Interfaces/BPI_Teams.I_SetTeam` _returnvalue_2 "NewEnumerator2")))))

(event `GetSpawnLocations`
  (bind _outactors (`GameplayStatics.GetAllActorsOfClass` "/Game/b014818k/Blueprints/BP_PlayerSpawn.BP_PlayerSpawn_C"))
  (set `self.SpawnLocations` _outactors))

(event `Spawn Characters`
  ;[0.2486 0.2218 1] Spawns Main Menu Characters
  (for _array_element (`self.Controllers`)
    (bind _spawn (`self.FindUnoccupiedSpawn`))
    (bind _returnvalue (`|SpawnActorFromClass` "/Game/b014818k/Blueprints/Characters/BasicPlayer/CH_BasicPlayer.CH_BasicPlayer_C" _spawn "AlwaysSpawn" "OverrideRootScale" null null))
    (message `/Game/b014818k/Blueprints/Interfaces/BPI_BaseGM.I_SetPawn` _array_element _returnvalue)
    (`Controller.Possess` _array_element _returnvalue)))

(event `Players Added`)

(event `self.ReceiveTick`
  (params (DeltaSeconds :type "Float (single-precision)")))

(fn `FindUnoccupiedSpawn`
  (returns (Spawn :type "Transform Structure"))
  (locals (FoundUnoccupiedSpawn :type Boolean :default true) (SpawnTransform :type "Transform Structure"))
  (bind _outitem (`KismetArrayLibrary.Array_Random` (`self.SpawnLocations`)))
  (while (`local.FoundUnoccupiedSpawn`)
    (if (not (`/Game/b014818k/Blueprints/BP_PlayerSpawn.IsValid` _outitem))
      (`KismetSystemLibrary.PrintString` (`KismetStringLibrary.Concat_StrStr` "Removed:" " " (`KismetSystemLibrary.GetDisplayName` _outitem)))
      (`KismetArrayLibrary.Array_RemoveItem` (`self.SpawnLocations`) _outitem)
      (else
        (`/Game/b014818k/Blueprints/BP_PlayerSpawn.SetSpawnInvalid` _outitem)
        (set `local.SpawnTransform` (`self.GetTransform` _outitem))
        (set `local.FoundUnoccupiedSpawn` false)
        (`KismetArrayLibrary.Array_RemoveItem` (`self.SpawnLocations`) _outitem)
        (return (`local.SpawnTransform`))))))

(fn `I_CheckSpawnLocationValid`
  (returns (Valid :type Boolean))
  (return false))

(fn `I_GetTeam`
  (returns (Team :type "/Game/b014818k/Blueprints/Enumerators/Enum_Teams Enum"))
  (return "NewEnumerator0"))

(fn `UserConstructionScript`)
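; BP_RotatingLog is a rotating log that switches between a default and a changed rotation rate through its RotatingMovement component.
; Unless the game mode reports Death Run through an interface call, chained timers alternate the two rates automatically from BeginPlay.
; IActivate applies the changed rate for a short time, blocking reactivation until a timer restores the default.
; It reports itself as a non-player through ICheckPlayer.
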(event `self.ReceiveBeginPlay`
  ;[0.08351 1 0.1068] If not deathrun gm, start automatic log rotation switch sequence.
  (set `RotatingMovementComponent.RotationRate` (`self.DefaultRotationRate`) (`self.RotatingMovement`))
  (bind _isdeathrungm (message `/Game/b014818k/Blueprints/Interfaces/BPI_DeathrunGM.I_IsDeathRunGM` (`GameplayStatics.GetGameMode`)))
  (if (not _isdeathrungm)
    (`KismetSystemLibrary.K2_SetTimerDelegate` (delegate `LogSwitchedOffAuto`) (`self.LogChangedRotationTime`) :!label _label)
    (set `RotatingMovementComponent.RotationRate` (`self.DefaultRotationRate`) (`self.RotatingMovement`))))

(event `LogSwitchedOnAuto`
  ;[0.08351 1 0.1068] If not deathrun gm, start automatic log rotation switch sequence.
  (goto _label))

(event `LogSwitchedOffAuto`
  ;[0.08351 1 0.1068] If not deathrun gm, start automatic log rotation switch sequence.
  (set `RotatingMovementComponent.RotationRate` (`self.ChangedRotationRate`) (`self.RotatingMovement`))
  (`KismetSystemLibrary.K2_SetTimer` null "LogSwitchedOnAuto" (`self.LogDefaultRotationTime`)))

(event `RotateTimer`
  ;[1 0.4962 0.2319] Changes the rotation of the log when activated, and after a short time goes back to the original rotation.
  (set `RotatingMovementComponent.RotationRate` (`self.DefaultRotationRate`) (`self.RotatingMovement`))
  (set `self.CanActivate` true))

(event `/Game/b014818k/Blueprints/Interfaces/BPI_Hit.I_Activate`
  (params (Activated :type Boolean))
  ;[1 0.4962 0.2319] Changes the rotation of the log when activated, and after a short time goes back to the original rotation.
  (if (`self.CanActivate`)
    (`KismetSystemLibrary.K2_SetTimerDelegate` (delegate `RotateTimer`) 5.0)
    (set `RotatingMovementComponent.RotationRate` (`self.ChangedRotationRate`) (`self.RotatingMovement`))
    (set `self.CanActivate` false)))

(fn `I_CheckPlayer`
  (returns (PlayerRef :type "Character Object Reference") (IsPlayer :type Boolean))
  (return null false))

(fn `UserConstructionScript`)
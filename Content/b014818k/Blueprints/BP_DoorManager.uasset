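; BP_DoorManager runs the doors and level transitions that trigger when all players are inside a checked area.
; It forwards player count to its door checkers, then reacts by the reporting checker's name.
; Gamemode checkers close one door, stream a sublevel (only race is named) and open the next door after a delay.
; Race checkers close a sublevel-registered door, then open TestMap with the RACE option on a timer.
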(event `/Game/b014818k/Blueprints/Interfaces/BPI_Door.I_SetSubLevelDoor`
  (params (Door :type "/Game/b014818k/Blueprints/BP_Door Object Reference"))
  (`KismetArrayLibrary.Array_Add` (`self.Level_Doors`) Door))

(event `/Game/b014818k/Blueprints/Interfaces/BPI_Door.I_SetNumberOfPlayers`
  (params (CurrentPlayers :type Integer))
  (set `self.PlayerAmount` CurrentPlayers)
  (for _array_element (`self.DoorCheckers`)
    (`/Game/b014818k/Blueprints/BP_DoorChecker.I_SetNumberOfPlayers` _array_element (`self.PlayerAmount`))))

(event `/Game/b014818k/Blueprints/Interfaces/BPI_Door.I_AllPlayersInside`
  (params (CheckerName :type String))
  (switch `string` CheckerName
    (:`BP_DoorChecker_2`
      ;[1 1 1] Load SubLevel: RaceGM
      (`self.GamemodeDoors` (`|GetArrayItem` (`self.Gamemode_Doors`)) (`|GetArrayItem` (`self.Gamemode_Doors`) 1))
      (`self.LoadSublevel` "StartingMap_RaceGM"))
    (:`BP_DoorChecker2`
      ;[1 1 1] Load SubLevel:
      (`self.GamemodeDoors` (`|GetArrayItem` (`self.Gamemode_Doors`) 2) (`|GetArrayItem` (`self.Gamemode_Doors`) 3))
      (`self.LoadSublevel` "None"))
    (:`BP_DoorChecker3`
      ;[1 1 1] Load SubLevel:
      (`self.GamemodeDoors` (`|GetArrayItem` (`self.Gamemode_Doors`) 4) (`|GetArrayItem` (`self.Gamemode_Doors`) 5))
      (`self.LoadSublevel` "None"))
    (:`BP_RaceGMCheck1`
      (`self.LevelDoors` (`|GetArrayItem` (`self.Level_Doors`)))
      (set `self.LevelToLoad` "TestMap")
      (`KismetSystemLibrary.K2_SetTimer` null "LoadNewGamemode" 3.0 :!label _label))
    (:`BP_RaceGMCheck2`
      (`self.LevelDoors` (`|GetArrayItem` (`self.Level_Doors`) 1))
      (set `self.LevelToLoad` "TestMap")
      (goto _label))
    (:`BP_RaceGMCheck3`
      (`self.LevelDoors` (`|GetArrayItem` (`self.Level_Doors`) 2))
      (set `self.LevelToLoad` "TestMap")
      (goto _label))))

(event `LoadNewGamemode`
  (`GameplayStatics.OpenLevel` (`self.LevelToLoad`) true "?RACE"))

(event `GamemodeDoors`
  (params (Door1 :type "/Game/b014818k/Blueprints/BP_Door Object Reference") (Door2 :type "/Game/b014818k/Blueprints/BP_Door Object Reference"))
  (`/Game/b014818k/Blueprints/BP_Door.I_CloseDoor` Door1)
  (`KismetSystemLibrary.K2_SetTimerDelegate` (delegate `OpenNextDoor`) 4.0))

(event `OpenNextDoor`
  (`/Game/b014818k/Blueprints/BP_Door.I_OpenDoor` (stale `GamemodeDoors` Door2)))

(event `LevelDoors`
  (params (Door :type "/Game/b014818k/Blueprints/BP_Door Object Reference"))
  (`/Game/b014818k/Blueprints/Interfaces/BPI_Door.I_CloseDoor` Door))

(event `LoadSublevel`
  (params (SublevelName :type Name))
  (`GameplayStatics.LoadStreamLevel` SublevelName true)
  (`KismetSystemLibrary.PrintString` (`KismetStringLibrary.Conv_NameToString` SublevelName)))

(fn `UserConstructionScript`)
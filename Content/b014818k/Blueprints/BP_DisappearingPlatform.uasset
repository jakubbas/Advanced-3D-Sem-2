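; Trap platform that disappears when activated through an interface event, removing the footing it provides until it reappears.
; Activation hides the actor, disables mesh collision and starts a one-shot timer that restores both after a few seconds.
; It works once per level attempt, since only the reset event re-arms it, also cancelling the timer and restoring the platform.
; Its player-check interface reports that it is not a player.
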(event `self.K2_OnReset`
  ;[0.2563 1 0.145] On level reset, allow the player to activate the trap again.
  (set `self.CanActivate` true)
  (`KismetSystemLibrary.K2_ClearAndInvalidateTimerHandle` (stale `/Game/b014818k/Blueprints/Interfaces/BPI_Hit.I_Activate` _returnvalue))
  (`self.SetActorHiddenInGame` false)
  (`PrimitiveComponent.SetCollisionEnabled` (`self.StaticMesh`) "QueryAndPhysics"))

(event `/Game/b014818k/Blueprints/Interfaces/BPI_Hit.I_Activate`
  (params (Activated :type Boolean))
  ;[1 0.1635 0.2332] Makes platform disappear on activation.
  (if (`self.CanActivate`)
    (bind _returnvalue (`KismetSystemLibrary.K2_SetTimerDelegate` (delegate `Reappear`) 5.0))
    (`self.SetActorHiddenInGame` true)
    (`PrimitiveComponent.SetCollisionEnabled` (`self.StaticMesh`) "NoCollision")
    (set `self.CanActivate` false)))

(event `Reappear`
  ;[0.08961 0 1] Makes the platforms reappear.
  (`self.SetActorHiddenInGame` false)
  (`PrimitiveComponent.SetCollisionEnabled` (`self.StaticMesh`) "QueryAndPhysics"))

(fn `I_CheckPlayer`
  (returns (PlayerRef :type "Character Object Reference") (IsPlayer :type Boolean))
  (return null false))

(fn `UserConstructionScript`)
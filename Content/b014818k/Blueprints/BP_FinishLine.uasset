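; BP_FinishLine is a race finish-line actor that reports to the game mode when a player reaches it.
; Its Box overlap asks the overlapping actor through an interface message whether it is a player, then sends that player's controller to the game mode through another interface message.
; It also contains stub interface functions for race game mode, player and score queries, which only return default values.
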(event `self.Box.OnComponentBeginOverlap`
  (params (OverlappedComponent :type "PrimitiveComponent Object Reference") (OtherActor :type "Actor Object Reference") (OtherComp :type "PrimitiveComponent Object Reference") (OtherBodyIndex :type Integer) (bFromSweep :type Boolean) (SweepResult :type "HitResult Structure (by ref)"))
  (bind (_playerref _isplayer) (message `/Game/b014818k/Blueprints/Interfaces/BPI_Hit.I_CheckPlayer` OtherActor))
  (if _isplayer
    (message `/Game/b014818k/Blueprints/Interfaces/BPI_RaceGM.I_PlayerReachedFinish` (`GameplayStatics.GetGameMode`) (`Pawn.GetController` _playerref))))

(fn `I_CheckForRaceGM`
  (returns (IsRaceGM :type Boolean))
  (return false))

(fn `I_CheckPlayer`
  (returns (PlayerRef :type "Character Object Reference") (IsPlayer :type Boolean))
  (return null false))

(fn `I_GetScore`
  (params (Controller :type "Controller Object Reference"))
  (returns (Score :type Integer))
  (return 0))

(fn `UserConstructionScript`)
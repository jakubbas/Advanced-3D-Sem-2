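; DeathBox is a trigger volume that sends a death message through an interface to any actor that begins overlapping its box.
; RaceGM, DeathRunGM and SumoGM flags can tie it to a game mode.
; On BeginPlay it queries the game mode for the first flag set, in that order, and destroys itself if the answer is false.
; With no flag set, it stays in every mode.
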(event `self.ReceiveBeginPlay`
  (if (or (`self.RaceGM`) (`self.DeathRunGM`) (`self.SumoGM`))
    (if (`self.RaceGM`)
      (bind _isracegm (message `/Game/b014818k/Blueprints/Interfaces/BPI_RaceGM.I_IsRaceGM` (`GameplayStatics.GetGameMode`)))
      (if (not _isracegm)
        (`self.K2_DestroyActor` self))
      (elif (`self.DeathRunGM`)
        (bind _isdeathrungm (message `/Game/b014818k/Blueprints/Interfaces/BPI_DeathrunGM.I_IsDeathRunGM` (`GameplayStatics.GetGameMode`)))
        (if (not _isdeathrungm)
          (`self.K2_DestroyActor` self))
        (else
          (bind _issumogm (message `/Game/b014818k/Blueprints/Interfaces/BPI_SumoGM.I_IsSumoGM` (`GameplayStatics.GetGameMode`)))
          (if (not _issumogm)
            (`self.K2_DestroyActor` self)))))))

(event `self.Box.OnComponentBeginOverlap`
  (params (OverlappedComponent :type "PrimitiveComponent Object Reference") (OtherActor :type "Actor Object Reference") (OtherComp :type "PrimitiveComponent Object Reference") (OtherBodyIndex :type Integer) (bFromSweep :type Boolean) (SweepResult :type "HitResult Structure (by ref)"))
  (message `/Game/b014818k/Blueprints/Interfaces/BPI_BasicPlayer.I_Death` OtherActor))

(fn `I_GetCharacter`
  (returns (Character :type "Character Object Reference"))
  (return null))

(fn `I_GetController`
  (returns (Controller :type "/Game/b014818k/Blueprints/Characters/BasicPlayer/PC_BasicPlayer Object Reference"))
  (return null))

(fn `UserConstructionScript`)
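; BP_SpinningPipe is a rotating pipe hazard that sends a death message to any player overlapping its Cylinder1 component.
; A RotatingMovement component spins it at a default rate, and IActivate switches to a changed rate for a few seconds before a timer restores it.
; CanActivate blocks retriggering until then.
; Player detection and death go through interface messages, and the pipe reports itself as non-player.
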(event `self.ReceiveBeginPlay`
  (set `RotatingMovementComponent.RotationRate` (`self.DefaultRotationRate`) (`self.RotatingMovement`)))

(event `self.Cylinder1.OnComponentBeginOverlap`
  (params (OverlappedComponent :type "PrimitiveComponent Object Reference") (OtherActor :type "Actor Object Reference") (OtherComp :type "PrimitiveComponent Object Reference") (OtherBodyIndex :type Integer) (bFromSweep :type Boolean) (SweepResult :type "HitResult Structure (by ref)"))
  (bind (_playerref _isplayer) (message `/Game/b014818k/Blueprints/Interfaces/BPI_Hit.I_CheckPlayer` OtherActor))
  (if _isplayer
    (message `/Game/b014818k/Blueprints/Interfaces/BPI_BasicPlayer.I_Death` _playerref)))

(event `/Game/b014818k/Blueprints/Interfaces/BPI_Hit.I_Activate`
  (params (Activated :type Boolean))
  (if (`self.CanActivate`)
    (set `RotatingMovementComponent.RotationRate` (`self.ChangedRotationRate`) (`self.RotatingMovement`))
    (set `self.CanActivate` false)
    (`KismetSystemLibrary.K2_SetTimerDelegate` (delegate `Timer`) 4.0)))

(event `Timer`
  (set `RotatingMovementComponent.RotationRate` (`self.DefaultRotationRate`) (`self.RotatingMovement`))
  (set `self.CanActivate` true))

(fn `I_CheckPlayer`
  (returns (PlayerRef :type "Character Object Reference") (IsPlayer :type Boolean))
  (return null false))

(fn `UserConstructionScript`)
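; BP_Pendulum is a swinging pendulum, apparently a trap, that runs automatically outside deathrun game modes.
; On BeginPlay it sets the RotatingMovement rate, waits a configurable delay, then plays SwingTimeline if the game mode's interface check reports no deathrun.
; SpikeSwitch auto events also drive the timelines, but their timer setup never runs and no timeline update logic is wired.
; It answers the ICheckPlayer interface as a non-player.
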(event `self.ReceiveBeginPlay`
  ;[0.2179 1 0] If the gamemode isn't deathrun, start the automatic spike sequence.
  (set `RotatingMovementComponent.RotationRate` (`self.DefaultRotationRate`) (`self.RotatingMovement`))
  (`KismetSystemLibrary.Delay` (`self.Delay`))
  (bind _isdeathrungm (message `/Game/b014818k/Blueprints/Interfaces/BPI_DeathrunGM.I_IsDeathRunGM` (`GameplayStatics.GetGameMode`)))
  (if (not _isdeathrungm)
    (`Timeline|SwingTimeline` :`NewTime` 0.5 :!via `PlayFromStart` :!label _label)))

(event `SpikeSwitchOnAuto`
  ;[0.2179 1 0] If the gamemode isn't deathrun, start the automatic spike sequence.
  (goto _label :!via `PlayFromStart`))

(event `SpikeSwitchOffAuto`
  ;[0.2179 1 0] If the gamemode isn't deathrun, start the automatic spike sequence.
  (`Timeline|SwingTimelineReverse` :`NewTime` 0.5 :!via `ReverseFromEnd`))

(fn `I_CheckPlayer`
  (returns (PlayerRef :type "Character Object Reference") (IsPlayer :type Boolean))
  (return null false))

(fn `UserConstructionScript`)
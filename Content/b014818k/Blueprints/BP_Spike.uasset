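; BP_Spike is a spike hazard that knocks the player away when its cone is hit, using a bounce component with configurable hit and upward force.
; It identifies the player through a check-player interface message and reports itself as a non-player.
; An activate interface call scales the cone along a timeline, then a timer plays a second scale timeline in reverse before re-enabling activation.
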(event `self.ReceiveBeginPlay`
  (set `self.DefaultScale` (`self.GetActorScale3D`)))

(event `self.Cone.OnComponentHit`
  (params (HitComponent :type "PrimitiveComponent Object Reference") (OtherActor :type "Actor Object Reference") (OtherComp :type "PrimitiveComponent Object Reference") (NormalImpulse :type "Vector Structure") (Hit :type "HitResult Structure (by ref)"))
  (bind (_playerref _isplayer) (message `/Game/b014818k/Blueprints/Interfaces/BPI_Hit.I_CheckPlayer` OtherActor))
  (if _isplayer
    (`/Game/b014818k/Blueprints/Components/BC_Bounce.BouncePlayer` (`self.BC_Bounce`) _playerref (`self.HitPower`) (`self.K2_GetActorLocation` self) (`self.UpPower`))))

(event `/Game/b014818k/Blueprints/Interfaces/BPI_Hit.I_Activate`
  (params (Activated :type Boolean))
  (if (`self.CanActivate`)
    (set `self.CanActivate` false)
    (bind (_direction _scale) (`Timeline|ScaleTimeline` :`NewTime` 0.5 :!via `PlayFromStart`)
      (:`Update`
        (`SceneComponent.SetWorldScale3D` (`self.Cone`) (* (`self.DefaultScale`) _scale)))
      (:`Finished`
        (set `self.DefaultScale` (`self.GetActorScale3D`))
        (`KismetSystemLibrary.K2_SetTimerDelegate` (delegate `Timer`) 4.0)))))

(event `Timer`
  (bind (_direction _scale) (`Timeline|ScaleReverse` :`NewTime` 0.5 :!via `ReverseFromEnd`)
    (:`Update`
      (`SceneComponent.SetWorldScale3D` (`self.Cone`) (* (`self.DefaultScale`) _scale)))
    (:`Finished`
      (set `self.CanActivate` true)
      (set `self.DefaultScale` (`self.GetActorScale3D`)))))

(fn `I_CheckPlayer`
  (returns (PlayerRef :type "Character Object Reference") (IsPlayer :type Boolean))
  (return null false))

(fn `UserConstructionScript`)
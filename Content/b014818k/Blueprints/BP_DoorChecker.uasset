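; BP_DoorChecker is a trigger volume that detects when the required number of players stand inside it.
; Collider overlaps match the actor against player pawns by index to raise or lower the count.
; Reaching the target notifies the level's BP_DoorManager once, through an interface call passing the checker's object name.
; An interface event updates the required count when the supplied number is equal or higher, so it never lowers it.
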(event `self.ReceiveBeginPlay`
  (bind _returnvalue (`GameplayStatics.GetActorOfClass` "/Game/b014818k/Blueprints/BP_DoorManager.BP_DoorManager_C"))
  (set `self.DoorManager` _returnvalue))

(event `self.Collider.OnComponentBeginOverlap`
  (params (OverlappedComponent :type "PrimitiveComponent Object Reference") (OtherActor :type "Actor Object Reference") (OtherComp :type "PrimitiveComponent Object Reference") (OtherBodyIndex :type Integer) (bFromSweep :type Boolean) (SweepResult :type "HitResult Structure (by ref)"))
  (bind _currentplayers (`self.CurrentPlayers`))
  (for _index (range (`self.RequiredPlayers`))
    (if (== OtherActor (`GameplayStatics.GetPlayerPawn` _index))
      (`/Engine/EditorBlueprintResources/StandardMacros.IncrementInt` _currentplayers
        (:`  `
          (if (== _currentplayers (`self.RequiredPlayers`))
            (`self.PlayersInside`)
            (break)
            (else
              (break))))))))

(event `self.Collider.OnComponentEndOverlap`
  (params (OverlappedComponent :type "PrimitiveComponent Object Reference") (OtherActor :type "Actor Object Reference") (OtherComp :type "PrimitiveComponent Object Reference") (OtherBodyIndex :type Integer))
  (for _index (range (`self.RequiredPlayers`))
    (if (== OtherActor (`GameplayStatics.GetPlayerPawn` _index))
      (`/Engine/EditorBlueprintResources/StandardMacros.DecrementInt` (`self.CurrentPlayers`)
        (:`  `
          (break))))))

(event `PlayersInside`
  (`/Engine/EditorBlueprintResources/StandardMacros.DoOnce` false
    (:`Completed`
      (`/Game/b014818k/Blueprints/Interfaces/BPI_Door.I_AllPlayersInside` (`self.DoorManager`) (`KismetSystemLibrary.GetObjectName` self)))))

(event `/Game/b014818k/Blueprints/Interfaces/BPI_Door.I_SetNumberOfPlayers`
  (params (CurrentPlayers :type Integer))
  (if (not (< CurrentPlayers (`self.RequiredPlayers`)))
    (set `self.RequiredPlayers` CurrentPlayers)))

(fn `UserConstructionScript`)
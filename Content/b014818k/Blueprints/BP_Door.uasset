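; BP_Door is a door that opens once, when the player pawn hits its DoorClosed component.
; A DoOnce gate then passes DoorClosed to OpenDoor and DoorOpen to CloseDoor, swapping the two parts vertically.
; Both custom events snap the given component to a preset relative Z with zero X and Y, without sweep or animation.
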(event `OpenDoor`
  (params (DoorReference :type "StaticMeshComponent Object Reference"))
  (`SceneComponent.K2_SetRelativeLocation` DoorReference (`KismetMathLibrary.MakeVector` 0.0 0.0 (`self.OpenZPos`)) false false))

(event `CloseDoor`
  (params (`Door Reference` :type "StaticMeshComponent Object Reference"))
  (`SceneComponent.K2_SetRelativeLocation` `Door Reference` (`KismetMathLibrary.MakeVector` 0.0 0.0 (`self.ClosedZPos`)) false false))

(event `self.DoorClosed.OnComponentHit`
  (params (HitComponent :type "PrimitiveComponent Object Reference") (OtherActor :type "Actor Object Reference") (OtherComp :type "PrimitiveComponent Object Reference") (NormalImpulse :type "Vector Structure") (Hit :type "HitResult Structure (by ref)"))
  (if (== OtherActor (`GameplayStatics.GetPlayerPawn` 0))
    (`/Engine/EditorBlueprintResources/StandardMacros.DoOnce` false
      (:`Completed`
        (`self.OpenDoor` (`self.DoorClosed`))
        (`self.CloseDoor` (`self.DoorOpen`))))))

(fn `UserConstructionScript`)